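; Card Blueprint for the Lucky Tester card, which adds a Lucky Tester projectile in DogFight.
; Its construction script chains a self-select instruction with an AddLuckyTester instruction and keeps a reference to the latter.
; GetCardDisplayInfo reads that instruction's upgradable damage, radius and test-fail ratio to build localized description items, using a custom Lucky Tester widget plus a follow-current-player buff line.
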(event EventBeginPlay)

(event Collision|EventActorBeginOverlap
  (params (OtherActor :type Actor%20Object%20Reference)))

(event EventTick
  (params (DeltaSeconds :type Float%20%28single-precision%29)))

(fn ConstructionScript
  (bind _self self)
  (bind _returnvalue (Game|ConstructObjectfromClass "/Script/CustomizableCard.InstructionSelectSelf" _self))
  (Class|CardBase|AddInstruction _returnvalue)
  (bind _returnvalue_2 (Game|ConstructObjectfromClass "/Game/DogFight/Blueprints/Cards/Instructions/Instruction_AddLuckyTester.Instruction_AddLuckyTester_C" _self))
  (Class|CardBase|AddInstruction _returnvalue_2)
  (Variables|Default|SetAddLuckyTesterInstruction _returnvalue_2))

(fn GetCardDisplayInfo
  (bind _carddisplayinfoargument (Utilities|Struct|MakeCardDisplayInfoArgument "Projectile" "Name_LuckyTester" "ILT_Projectile" false))
  (bind _descriptionitems (LocalVariables|GetDescriptionItems))
  (bind _addluckytesterinstruction (Variables|Default|GetAddLuckyTesterInstruction))
  (bind _damage (Variables|/Script/DogFight.InstructionAddLuckyTester|GetDamage _addluckytesterinstruction))
  (bind _damageradius (Variables|/Script/DogFight.InstructionAddLuckyTester|GetDamageRadius _addluckytesterinstruction))
  (bind _testfailradio (Variables|/Script/DogFight.InstructionAddLuckyTester|GetTestFailRadio _addluckytesterinstruction))
  (Utilities|Array|Clear (LocalVariables|GetDescriptionItems))
  (Utilities|Array|Add _descriptionitems (Utilities|Struct|MakeCardDescriptionItemInfo "Desc_LuckyTester" 0 (Utilities|Array|MakeArray _carddisplayinfoargument (Utilities|Struct|MakeCardDisplayInfoArgument "Default" (Utilities|String|ToString(Integer) (Class|CardBase|GetUpgradableIntPropertyValue _damage)) "ILT_Raw" false) (Utilities|Struct|MakeCardDisplayInfoArgument "Default" "PhysicalDamage" "ILT_Raw" true) (Utilities|Struct|MakeCardDisplayInfoArgument "Default" (Utilities|String|ToString(Integer) (Class|CardBase|GetUpgradableIntPropertyValue _damageradius)) "ILT_Raw" false) (Utilities|Struct|MakeCardDisplayInfoArgument "Default" (Class|CardBase|GetUpgradableFloatPropertyValue _testfailradio) "ILT_Raw" false)) "ILT_Projectile" "/Game/DogFight/UI/InGame/CardDisplay/BP_CardDescriptionLuckyTesterItem.BP_CardDescriptionLuckyTesterItem_C" (Utilities|Array|MakeArray (Class|CardBase|GetIntPropertyDisplayInfo _damage) (Class|CardBase|GetIntPropertyDisplayInfo _damageradius) (Class|CardBase|GetFloatPropertyDisplayInfo _testfailradio))))
  (Utilities|Array|Add _descriptionitems (Utilities|Struct|MakeCardDescriptionItemInfo "Desc_FollowCurrentPlayer" 0 0 "ILT_Buff" "/Game/DogFight/UI/InGame/CardDisplay/BP_CardDescriptionItemWidget.BP_CardDescriptionItemWidget_C"))
  (return (Utilities|Struct|MakeCardInstanceDisplayInfo (Variables|Default|GetCardName) (Utilities|Array|MakeArray (Utilities|Struct|MakeCardDisplayInfoArgument "Projectile" "Name_LuckyTester" "ILT_Projectile" true)) (Variables|Default|GetCardDescription) (Utilities|Array|MakeArray _carddisplayinfoargument) (LocalVariables|GetDescriptionItems))))