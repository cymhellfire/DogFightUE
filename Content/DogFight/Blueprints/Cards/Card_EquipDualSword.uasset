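; Card Blueprint in DogFight that equips the Dual Sword weapon on the user.
; Its construction script queues two instructions: InstructionSelectSelf to target the user, then Instruction_EquipDualSword.
; GetCardDisplayInfo fills the card name and description with localized weapon arguments and adds a Dual Sword detail item shown through BP_CardDescriptionWeaponItemWidget.
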(event EventBeginPlay)

(event Collision|EventActorBeginOverlap
  (params (OtherActor :type Actor%20Object%20Reference)))

(event EventTick
  (params (DeltaSeconds :type Float%20%28single-precision%29)))

(fn ConstructionScript
  (bind _returnvalue (Game|ConstructObjectfromClass "/Script/DogFight.InstructionSelectSelf" self))
  (Class|CardBase|AddInstruction _returnvalue)
  (bind _returnvalue_2 (Game|ConstructObjectfromClass "/Game/DogFight/Blueprints/Cards/Instructions/Instruction_EquipDualSword.Instruction_EquipDualSword_C" self))
  (Class|CardBase|AddInstruction _returnvalue_2))

(fn GetCardDisplayInfo
  (bind _carddisplayinfoargument (Utilities|Struct|MakeCardDisplayInfoArgument "Projectile" "Weapon_DualSword" "ILT_Weapon" false))
  (return (Utilities|Struct|MakeCardInstanceDisplayInfo (Variables|Default|GetCardName) (Utilities|Array|MakeArray (Utilities|Struct|MakeCardDisplayInfoArgument "Default" "Weapon_DualSword" "ILT_Weapon" true)) (Variables|Default|GetCardDescription) (Utilities|Array|MakeArray _carddisplayinfoargument) (Utilities|Array|MakeArray (Utilities|Struct|MakeCardDescriptionItemInfo "Desc_DualSword" 0 (Utilities|Array|MakeArray _carddisplayinfoargument (Utilities|Struct|MakeCardDisplayInfoArgument "Default" "DualSword" "ILT_Raw" true)) "ILT_Weapon" "/Game/DogFight/UI/InGame/CardDisplay/BP_CardDescriptionWeaponItemWidget.BP_CardDescriptionWeaponItemWidget_C")))))