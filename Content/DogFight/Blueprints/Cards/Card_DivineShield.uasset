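; Card_DivineShield is a card Blueprint that grants one Divine Shield buff, an invincibility effect, to a selected actor.
; Construction builds its instruction chain: a single-actor selection step, then an Add Invincible step kept as a variable.
; GetCardDisplayInfo supplies localized name and description arguments plus a shield detail item, whose text key follows that instruction's shield block type (Enemy, Ally, NotMine or All).
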(event EventBeginPlay)

(event Collision|EventActorBeginOverlap
  (params (OtherActor :type Actor%20Object%20Reference)))

(event EventTick
  (params (DeltaSeconds :type Float%20%28single-precision%29)))

(fn ConstructionScript
  (bind _returnvalue (Game|ConstructObjectfromClass "/Game/DogFight/Blueprints/Cards/Instructions/Instruction_SelectOneActor.Instruction_SelectOneActor_C" self))
  (Class|CardBase|AddInstruction _returnvalue)
  (bind _returnvalue_2 (Game|ConstructObjectfromClass "/Game/DogFight/Blueprints/Cards/Instructions/Instruction_AddInvincible.Instruction_AddInvincible_C" self))
  (Variables|Default|SetAddInvincibleInstruction _returnvalue_2)
  (Class|CardBase|AddInstruction _returnvalue_2))

(fn GetCardDisplayInfo
  (bind _carddisplayinfoargument (Utilities|Struct|MakeCardDisplayInfoArgument "Buff" "Name_DivineShield" "ILT_Buff" false))
  (bind _carddisplayinfoargument_2 (Utilities|Struct|MakeCardDisplayInfoArgument "Default" "1" "ILT_Raw" false))
  (return (Utilities|Struct|MakeCardInstanceDisplayInfo (Variables|Default|GetCardName) (Utilities|Array|MakeArray (Utilities|Struct|MakeCardDisplayInfoArgument "Buff" "Name_DivineShield" "ILT_Buff" true) _carddisplayinfoargument_2) (Variables|Default|GetCardDescription) (Utilities|Array|MakeArray _carddisplayinfoargument _carddisplayinfoargument_2) (Utilities|Array|MakeArray (Utilities|Struct|MakeCardDescriptionItemInfo "Desc_DivineShield" (Utilities|Array|MakeArray (Utilities|Struct|MakeCardDisplayInfoArgument "Default" (Utilities|Select :Index (Variables|/Script/CustomizableCard.InstructionPlaceShield|GetShieldBlockType (Variables|Default|GetAddInvincibleInstruction)) :SBT_Enemy "Param_DivineShield_Enemy" :SBT_Ally "Param_DivineShield_Ally" :SBT_NotMine "Param_DivineShield_NotMine" :SBT_All "Param_DivineShield_All") "ILT_Buff" false)) (Utilities|Array|MakeArray _carddisplayinfoargument) "ILT_Buff" "/Game/DogFight/UI/InGame/BP_CardDescriptionShieldItem.BP_CardDescriptionShieldItem_C")))))