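; Card Blueprint for the Nuclear Strike card, which carries a nuclear missile attack.
; Construction adds a random-one-point instruction followed by a NuclearStrike instruction, keeping a reference to the latter.
; GetCardDisplayInfo reads that instruction's upgradable damage, speed and radius into a localized projectile description, then appends each enhancement's description and name prefix.
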(event EventBeginPlay)

(event Collision|EventActorBeginOverlap
  (params (OtherActor :type Actor%20Object%20Reference)))

(event EventTick
  (params (DeltaSeconds :type Float%20%28single-precision%29)))

(fn ConstructionScript
  (bind _returnvalue (Game|ConstructObjectfromClass "/Game/DogFight/Blueprints/Cards/Instructions/Instruction_RandomOnePoint.Instruction_RandomOnePoint_C" self))
  (Class|CardBase|AddInstruction _returnvalue)
  (bind _returnvalue_2 (Game|ConstructObjectfromClass "/Game/DogFight/Blueprints/Cards/Instructions/Instruction_NuclearStrike.Instruction_NuclearStrike_C" self))
  (Variables|Default|SetNuclearStrikeInstruction _returnvalue_2)
  (Class|CardBase|AddInstruction _returnvalue_2))

(fn GetCardDisplayInfo
  (bind _carddisplayinfoargument (Utilities|Struct|MakeCardDisplayInfoArgument "Projectile" "Name_NuclearMissile" "ILT_Projectile"))
  (bind _nuclearstrikeinstruction (Variables|Default|GetNuclearStrikeInstruction))
  (bind _initialspeed (Variables|/Script/CustomizableCard.InstructionSpawnProjectileAt|GetInitialSpeed _nuclearstrikeinstruction))
  (bind _damageradius (Variables|/Script/CustomizableCard.InstructionSpawnProjectileAt|GetDamageRadius _nuclearstrikeinstruction))
  (bind _damage (Variables|/Script/CustomizableCard.InstructionSpawnProjectileAt|GetDamage _nuclearstrikeinstruction))
  (Utilities|Array|Clear (LocalVariables|GetDescriptionItems))
  (Utilities|Array|Add (LocalVariables|GetDescriptionItems) (Utilities|Struct|MakeCardDescriptionItemInfo "Desc_NuclearMissile" 0 (Utilities|Array|MakeArray _carddisplayinfoargument (Utilities|Struct|MakeCardDisplayInfoArgument "Default" (Utilities|String|ToString(Integer) (Class|CardBase|GetUpgradablePropertyValue _damage)) "ILT_Raw") (Utilities|Struct|MakeCardDisplayInfoArgument "Default" "PhysicalDamage" "ILT_RawNoStyle") (Utilities|Struct|MakeCardDisplayInfoArgument "Default" (Utilities|String|ToString(Integer) (Class|CardBase|GetUpgradablePropertyValue _initialspeed)) "ILT_Raw") (Utilities|Struct|MakeCardDisplayInfoArgument "Default" (Utilities|String|ToString(Integer) (Class|CardBase|GetUpgradablePropertyValue _damageradius)) "ILT_Raw")) "ILT_Projectile" "/Game/DogFight/UI/InGame/BP_CardDescriptionProjectileItemWidget.BP_CardDescriptionProjectileItemWidget_C" (Utilities|Array|MakeArray (Class|CardBase|GetPropertyDisplayInfo _damage) (Class|CardBase|GetPropertyDisplayInfo _initialspeed) (Class|CardBase|GetPropertyDisplayInfo _damageradius))))
  ;[1 1 1] Add all enhancement description
  (for _array_element (Variables|Default|GetCardEnhancements)
    (bind _returnvalue (Class|CardEnhancement|GetDescriptionItemInfo _array_element))
    (Utilities|Array|Add (LocalVariables|GetDescriptionItems) _returnvalue)
    (Utilities|Array|Add (LocalVariables|GetEnhancePrefix) (Variables|/Script/CustomizableCard.CardEnhancement|GetEnhancementPrefix _array_element)))
  (return (Utilities|Struct|MakeCardInstanceDisplayInfo (Variables|Default|GetCardName) (Utilities|Array|MakeArray _carddisplayinfoargument) (Variables|Default|GetCardDescription) (Utilities|Array|MakeArray _carddisplayinfoargument) (LocalVariables|GetDescriptionItems) (LocalVariables|GetEnhancePrefix))))