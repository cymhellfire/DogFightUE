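; Fireball card for the DogFight game that targets one actor and launches a fireball projectile.
; The construction script chains a select-one-actor instruction and a fireball instruction, then applies and registers damage-level and projectile-speed enhancements on the fireball.
; GetCardDisplayInfo builds localized card text from the fireball's upgradable damage, muzzle speed and radius, appending each enhancement's description and name prefix.
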(event EventBeginPlay)

(event Collision|EventActorBeginOverlap
  (params (OtherActor :type Actor%20Object%20Reference)))

(event EventTick
  (params (DeltaSeconds :type Float%20%28single-precision%29)))

(fn ConstructionScript
  (bind _returnvalue (Game|ConstructObjectfromClass "/Game/DogFight/Blueprints/Cards/Instructions/Instruction_SelectOneActor.Instruction_SelectOneActor_C" self))
  (Class|CardBase|AddInstruction _returnvalue)
  (bind _returnvalue_2 (Game|ConstructObjectfromClass "/Game/DogFight/Blueprints/Cards/Instructions/Instruction_Fireball.Instruction_Fireball_C" self))
  (Variables|Default|SetFireballInstruction _returnvalue_2)
  (Class|CardBase|AddInstruction _returnvalue_2)
  (bind _returnvalue_3 (Game|ConstructObjectfromClass "/Game/DogFight/Blueprints/Cards/CardEnhancements/BP_EnhanceDamageLevel.BP_EnhanceDamageLevel_C" self))
  (Class|InstructionPropertyEnhancement|SetTargetInstruction _returnvalue_3 (Variables|Default|GetFireballInstruction))
  (Class|InstructionPropertyEnhancement|ApplyEnhancement _returnvalue_3)
  (Class|CardBase|AddCardEnhancement _returnvalue_3)
  (bind _returnvalue_4 (Game|ConstructObjectfromClass "/Game/DogFight/Blueprints/Cards/CardEnhancements/BP_EnhanceProjectileSpeedLevel.BP_EnhanceProjectileSpeedLevel_C" self))
  (Class|InstructionPropertyEnhancement|SetTargetInstruction _returnvalue_4 (Variables|Default|GetFireballInstruction))
  (Class|InstructionPropertyEnhancement|ApplyEnhancement _returnvalue_4)
  (Class|CardBase|AddCardEnhancement _returnvalue_4))

(fn GetCardDisplayInfo
  (bind _carddisplayinfoargument (Utilities|Struct|MakeCardDisplayInfoArgument "Projectile" "Name_Fireball" "ILT_Projectile"))
  (bind _fireballinstruction (Variables|Default|GetFireballInstruction))
  (bind _damageradius (Variables|/Script/CustomizableCard.InstructionFireProjectile|GetDamageRadius _fireballinstruction))
  (bind _damage (Variables|/Script/CustomizableCard.InstructionFireProjectile|GetDamage _fireballinstruction))
  (bind _muzzlespeed (Variables|/Script/CustomizableCard.InstructionFireProjectile|GetMuzzleSpeed _fireballinstruction))
  (Utilities|Array|Clear (LocalVariables|GetDescriptionItems))
  (Utilities|Array|Add (LocalVariables|GetDescriptionItems) (Utilities|Struct|MakeCardDescriptionItemInfo "Desc_Fireball" 0 (Utilities|Array|MakeArray _carddisplayinfoargument (Utilities|Struct|MakeCardDisplayInfoArgument "Default" (Utilities|String|ToString(Integer) (Class|CardBase|GetUpgradablePropertyValue _damage)) "ILT_Raw") (Utilities|Struct|MakeCardDisplayInfoArgument "Default" "FireDamage" "ILT_RawNoStyle") (Utilities|Struct|MakeCardDisplayInfoArgument "Default" (Utilities|String|ToString(Integer) (Class|CardBase|GetUpgradablePropertyValue _muzzlespeed)) "ILT_Raw") (Utilities|Struct|MakeCardDisplayInfoArgument "Default" (Utilities|String|ToString(Integer) (Class|CardBase|GetUpgradablePropertyValue _damageradius)) "ILT_Raw")) "ILT_Projectile" "/Game/DogFight/UI/InGame/BP_CardDescriptionProjectileItemWidget.BP_CardDescriptionProjectileItemWidget_C" (Utilities|Array|MakeArray (Class|CardBase|GetPropertyDisplayInfo _damage) (Class|CardBase|GetPropertyDisplayInfo _muzzlespeed) (Class|CardBase|GetPropertyDisplayInfo _damageradius))))
  ;[1 1 1] Add all enhancement description
  (for _array_element (Variables|Default|GetCardEnhancements)
    (bind _returnvalue (Class|CardEnhancement|GetDescriptionItemInfo _array_element))
    (Utilities|Array|Add (LocalVariables|GetDescriptionItems) _returnvalue)
    (Utilities|Array|Add (LocalVariables|GetEnhancePrefix) (Variables|/Script/CustomizableCard.CardEnhancement|GetEnhancementPrefix _array_element)))
  (return (Utilities|Struct|MakeCardInstanceDisplayInfo (Variables|Default|GetCardName) (Utilities|Array|MakeArray _carddisplayinfoargument) (Variables|Default|GetCardDescription) (Utilities|Array|MakeArray _carddisplayinfoargument) (LocalVariables|GetDescriptionItems) (LocalVariables|GetEnhancePrefix))))