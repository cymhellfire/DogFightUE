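; Card Blueprint for DogFight that applies a Physical Armor buff to one selected actor.
; The construction script composes it from two instructions: a single-actor selection, then a BP_AddPhysicalArmorBuff kept as AddArmorInstruction.
; GetCardDisplayInfo builds localized name and description arguments with a hard-coded count, plus an armor tooltip item that reads the instruction's upgradable ArmorValue.
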(event EventBeginPlay)

(event Collision|EventActorBeginOverlap
  (params (OtherActor :type Actor%20Object%20Reference)))

(event EventTick
  (params (DeltaSeconds :type Float%20%28single-precision%29)))

(fn ConstructionScript
  (bind _returnvalue (Game|ConstructObjectfromClass "/Game/DogFight/Blueprints/Cards/Instructions/Instruction_SelectOneActor.Instruction_SelectOneActor_C" self))
  (Class|CardBase|AddInstruction _returnvalue)
  (bind _returnvalue_2 (Game|ConstructObjectfromClass "/Game/DogFight/Blueprints/Cards/Instructions/BP_AddPhysicalArmorBuff.BP_AddPhysicalArmorBuff_C" self))
  (Variables|Default|SetAddArmorInstruction _returnvalue_2)
  (Class|CardBase|AddInstruction _returnvalue_2))

(fn GetCardDisplayInfo
  (bind _carddisplayinfoargument (Utilities|Struct|MakeCardDisplayInfoArgument "Default" "1" "ILT_Raw" false))
  (bind _addarmorinstruction (Variables|Default|GetAddArmorInstruction))
  (bind _armorvalue (Variables|/Script/DogFight.InstructionAddArmor|GetArmorValue _addarmorinstruction))
  (return (Utilities|Struct|MakeCardInstanceDisplayInfo (Variables|Default|GetCardName) (Utilities|Array|MakeArray (Utilities|Struct|MakeCardDisplayInfoArgument "Buff" "Name_PhysicalArmor" "ILT_Buff" true) _carddisplayinfoargument) (Variables|Default|GetCardDescription) (Utilities|Array|MakeArray (Utilities|Struct|MakeCardDisplayInfoArgument "Buff" "Name_PhysicalArmor" "ILT_Buff" false) _carddisplayinfoargument) (Utilities|Array|MakeArray (Utilities|Struct|MakeCardDescriptionItemInfo "Desc_PhysicalArmor" 0 (Utilities|Array|MakeArray (Utilities|Struct|MakeCardDisplayInfoArgument "Buff" "Name_PhysicalArmor" "ILT_Buff" false) (Utilities|Struct|MakeCardDisplayInfoArgument "Default" (Utilities|String|ToString(Integer) (Class|CardBase|GetUpgradableIntPropertyValue _armorvalue)) "ILT_Raw" false) (Utilities|Struct|MakeCardDisplayInfoArgument "Default" "PhysicalArmor" "ILT_Raw" true)) "ILT_Buff" "/Game/DogFight/UI/InGame/CardDisplay/BP_CardDescriptionArmorBuffItemWidget.BP_CardDescriptionArmorBuffItemWidget_C" (Utilities|Array|MakeArray (Class|CardBase|GetIntPropertyDisplayInfo _armorvalue)))))))