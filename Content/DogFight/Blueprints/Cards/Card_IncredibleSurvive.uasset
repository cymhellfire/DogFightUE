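; Card in DogFight that gives the Incredible Survive buff to its own user.
; The construction script queues two instructions: one selects self, the next adds the buff.
; GetCardDisplayInfo fills the name and description with hardcoded buff arguments, and appends a buff detail item shown through a dedicated description widget.
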(event EventBeginPlay)

(event Collision|EventActorBeginOverlap
  (params (OtherActor :type Actor%20Object%20Reference)))

(event EventTick
  (params (DeltaSeconds :type Float%20%28single-precision%29)))

(fn ConstructionScript
  (bind _returnvalue (Game|ConstructObjectfromClass "/Script/DogFight.InstructionSelectSelf" self))
  (Class|CardBase|AddInstruction _returnvalue)
  (bind _returnvalue_2 (Game|ConstructObjectfromClass "/Game/DogFight/Blueprints/Cards/Instructions/Instruction_AddIncredibleSurvive.Instruction_AddIncredibleSurvive_C" self))
  (Class|CardBase|AddInstruction _returnvalue_2))

(fn GetCardDisplayInfo
  (bind _carddisplayinfoargument (Utilities|Struct|MakeCardDisplayInfoArgument "Buff" "Name_IncredibleSurvive" "ILT_Buff" false))
  (bind _carddisplayinfoargument_2 (Utilities|Struct|MakeCardDisplayInfoArgument "Default" "1" "ILT_Raw" false))
  (return (Utilities|Struct|MakeCardInstanceDisplayInfo (Variables|Default|GetCardName) (Utilities|Array|MakeArray (Utilities|Struct|MakeCardDisplayInfoArgument "Buff" "Name_IncredibleSurvive" "ILT_Buff" true) _carddisplayinfoargument_2) (Variables|Default|GetCardDescription) (Utilities|Array|MakeArray _carddisplayinfoargument _carddisplayinfoargument_2) (Utilities|Array|MakeArray (Utilities|Struct|MakeCardDescriptionItemInfo "Desc_IncredibleSurvive" (Utilities|Array|MakeArray (Utilities|Struct|MakeCardDisplayInfoArgument "Default" "10%" "ILT_Raw" false) (Utilities|Struct|MakeCardDisplayInfoArgument "Default" "100%" "ILT_Raw" false)) (Utilities|Array|MakeArray _carddisplayinfoargument) "ILT_Buff" "/Game/DogFight/UI/InGame/CardDisplay/BP_CardDescriptionIncredibleSurviveBuffItemWidget.BP_CardDescriptionIncredibleSurviveBuffItemWidget_C")))))