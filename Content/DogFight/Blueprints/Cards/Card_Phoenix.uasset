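; Phoenix card for DogFight that selects half the players and summons a phoenix.
; The construction script composes it from two instruction objects, a half-player selection followed by the summon, and keeps a reference to the summon instruction.
; Its display info reads that instruction's upgradable total damage to fill a localized description shown through a Phoenix-specific item widget.
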(event EventBeginPlay)

(event Collision|EventActorBeginOverlap
  (params (OtherActor :type Actor%20Object%20Reference)))

(event EventTick
  (params (DeltaSeconds :type Float%20%28single-precision%29)))

(fn ConstructionScript
  (bind _returnvalue (Game|ConstructObjectfromClass "/Game/DogFight/Blueprints/Cards/Instructions/Instruction_SelectHalfPlayers.Instruction_SelectHalfPlayers_C" self))
  (Class|CardBase|AddInstruction _returnvalue)
  (bind _returnvalue_2 (Game|ConstructObjectfromClass "/Game/DogFight/Blueprints/Cards/Instructions/Instruction_SummonPhoenix.Instruction_SummonPhoenix_C" self))
  (Variables|Default|SetPhoenixInstruction _returnvalue_2)
  (Class|CardBase|AddInstruction _returnvalue_2))

(fn GetCardDisplayInfo
  (bind _phoenixinstruction (Variables|Default|GetPhoenixInstruction))
  (bind _totaldamage (Variables|/Script/DogFight.InstructionSummonPhoenix|GetTotalDamage _phoenixinstruction))
  (return (Utilities|Struct|MakeCardInstanceDisplayInfo (Variables|Default|GetCardName) 0 (Variables|Default|GetCardDescription) 0 (Utilities|Array|MakeArray (Utilities|Struct|MakeCardDescriptionItemInfo "Desc_Phoenix" 0 (Utilities|Array|MakeArray (Utilities|Struct|MakeCardDisplayInfoArgument "Default" (Utilities|String|ToString(Integer) (Class|CardBase|GetUpgradableIntPropertyValue _totaldamage)) "ILT_Raw" false) (Utilities|Struct|MakeCardDisplayInfoArgument "Projectile" "Name_Phoenix" "ILT_Projectile" false)) "ILT_Projectile" "/Game/DogFight/UI/InGame/CardDisplay/BP_CardDescriptionPhoenixItemWidget.BP_CardDescriptionPhoenixItemWidget_C" (Utilities|Array|MakeArray (Class|CardBase|GetIntPropertyDisplayInfo _totaldamage)))))))