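; Fool card for DogFight that selects one actor and applies a Skip Use Card effect.
; The construction script composes the card from two instruction objects, target selection followed by adding the skip, rather than custom event logic.
; GetCardDisplayInfo supplies the name and description with localized buff arguments, plus an extra description item explaining the buff through a dedicated skip-phase widget.
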(event EventBeginPlay)

(event Collision|EventActorBeginOverlap
  (params (OtherActor :type Actor%20Object%20Reference)))

(event EventTick
  (params (DeltaSeconds :type Float%20%28single-precision%29)))

(fn ConstructionScript
  (bind _returnvalue (Game|ConstructObjectfromClass "/Game/DogFight/Blueprints/Cards/Instructions/Instruction_SelectOneActor.Instruction_SelectOneActor_C" self))
  (Class|CardBase|AddInstruction _returnvalue)
  (bind _returnvalue_2 (Game|ConstructObjectfromClass "/Game/DogFight/Blueprints/Cards/Instructions/Instruction_AddSkipUseCard.Instruction_AddSkipUseCard_C" self))
  (Class|CardBase|AddInstruction _returnvalue_2))

(fn GetCardDisplayInfo
  (bind _carddisplayinfoargument (Utilities|Struct|MakeCardDisplayInfoArgument "Buff" "Name_SkipUseCard" "ILT_Buff" false))
  (bind _carddisplayinfoargument_2 (Utilities|Struct|MakeCardDisplayInfoArgument "Default" "1" "ILT_Raw" true))
  (return (Utilities|Struct|MakeCardInstanceDisplayInfo (Variables|Default|GetCardName) (Utilities|Array|MakeArray _carddisplayinfoargument_2) (Variables|Default|GetCardDescription) (Utilities|Array|MakeArray _carddisplayinfoargument _carddisplayinfoargument_2) (Utilities|Array|MakeArray (Utilities|Struct|MakeCardDescriptionItemInfo "Desc_SkipUseCard" 0 (Utilities|Array|MakeArray _carddisplayinfoargument) "ILT_Buff" "/Game/DogFight/UI/InGame/CardDisplay/BP_CardDescriptionSkipGamePhaseBuffItemWidget.BP_CardDescriptionSkipGamePhaseBuffItemWidget_C")))))