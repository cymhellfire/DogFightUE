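; Card_Chaos is a DogFight card that applies the Chaos buff to a selected actor.
; The construction script chains a select-one-actor instruction with an add-chaos instruction, keeping the latter for display.
; GetCardDisplayInfo builds the localized name and description with a fixed amount of one.
; An extra Chaos buff description item shows the upgradable chaos possibility read from that instruction, using a dedicated item widget.
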(event EventBeginPlay)

(event Collision|EventActorBeginOverlap
  (params (OtherActor :type Actor%20Object%20Reference)))

(event EventTick
  (params (DeltaSeconds :type Float%20%28single-precision%29)))

(fn ConstructionScript
  (bind _returnvalue (Game|ConstructObjectfromClass "/Game/DogFight/Blueprints/Cards/Instructions/Instruction_SelectOneActor.Instruction_SelectOneActor_C" self))
  (Class|CardBase|AddInstruction _returnvalue)
  (bind _returnvalue_2 (Game|ConstructObjectfromClass "/Game/DogFight/Blueprints/Cards/Instructions/Instruction_AddChaos.Instruction_AddChaos_C" self))
  (Variables|Default|SetAddChaosInstruction _returnvalue_2)
  (Class|CardBase|AddInstruction _returnvalue_2))

(fn GetCardDisplayInfo
  (bind _carddisplayinfoargument (Utilities|Struct|MakeCardDisplayInfoArgument "Buff" "Name_Chaos" "ILT_Buff" false))
  (bind _carddisplayinfoargument_2 (Utilities|Struct|MakeCardDisplayInfoArgument "Default" "1" "ILT_Raw" true))
  (bind _addchaosinstruction (Variables|Default|GetAddChaosInstruction))
  (bind _chaospossibility (Variables|/Script/DogFight.InstructionAddChaos|GetChaosPossibility _addchaosinstruction))
  (return (Utilities|Struct|MakeCardInstanceDisplayInfo (Variables|Default|GetCardName) (Utilities|Array|MakeArray (Utilities|Struct|MakeCardDisplayInfoArgument "Buff" "Name_Chaos" "ILT_Buff" true) _carddisplayinfoargument_2) (Variables|Default|GetCardDescription) (Utilities|Array|MakeArray _carddisplayinfoargument _carddisplayinfoargument_2) (Utilities|Array|MakeArray (Utilities|Struct|MakeCardDescriptionItemInfo "Desc_Chaos" 0 (Utilities|Array|MakeArray _carddisplayinfoargument (Utilities|Struct|MakeCardDisplayInfoArgument "Default" (Class|CardBase|GetUpgradableFloatPropertyValue _chaospossibility) "ILT_Raw" true)) "ILT_Buff" "/Game/DogFight/UI/InGame/CardDisplay/BP_CardDescriptionChaosBuffItemWidget.BP_CardDescriptionChaosBuffItemWidget_C" (Utilities|Array|MakeArray (Class|CardBase|GetFloatPropertyDisplayInfo _chaospossibility)))))))