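; Card Blueprint for a steal-card card in DogFight that takes cards from a selected actor.
; The construction script chains a select-one-actor instruction and a steal-cards instruction, keeping a reference to the latter.
; GetCardDisplayInfo feeds the steal instruction's upgradable card count into the name, description and a steal-action detail item with its own widget.
; The event graph holds only disabled stub events.
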(event EventBeginPlay)

(event Collision|EventActorBeginOverlap
  (params (OtherActor :type Actor%20Object%20Reference)))

(event EventTick
  (params (DeltaSeconds :type Float%20%28single-precision%29)))

(fn ConstructionScript
  (bind _returnvalue (Game|ConstructObjectfromClass "/Game/DogFight/Blueprints/Cards/Instructions/Instruction_SelectOneActor.Instruction_SelectOneActor_C" self))
  (Class|CardBase|AddInstruction _returnvalue)
  (bind _returnvalue_2 (Game|ConstructObjectfromClass "/Game/DogFight/Blueprints/Cards/Instructions/Instruction_StealCards.Instruction_StealCards_C" self))
  (bind _output_get (Variables|Default|SetStealCardInstruction _returnvalue_2))
  (Class|CardBase|AddInstruction _output_get))

(fn GetCardDisplayInfo
  (bind _stealcardinstruction (Variables|Default|GetStealCardInstruction))
  (bind _cardcount (Variables|/Script/DogFight.InstructionStealCard|GetCardCount _stealcardinstruction))
  (bind _returnvalue (Class|CardBase|GetUpgradableIntPropertyValue _cardcount))
  (bind _returnvalue_2 (Utilities|String|ToString(Integer) _returnvalue))
  (bind _carddisplayinfoargument (Utilities|Struct|MakeCardDisplayInfoArgument "Default" _returnvalue_2 "ILT_Raw" true))
  (bind _array (Utilities|Array|MakeArray _carddisplayinfoargument))
  (return (Utilities|Struct|MakeCardInstanceDisplayInfo (Variables|Default|GetCardName) _array (Variables|Default|GetCardDescription) _array (Utilities|Array|MakeArray (Utilities|Struct|MakeCardDescriptionItemInfo "Desc_StealCardAction" 0 (Utilities|Array|MakeArray (Utilities|Struct|MakeCardDisplayInfoArgument "Buff" "Name_StealCardAction" "ILT_Card" false) _carddisplayinfoargument) "ILT_Card" "/Game/DogFight/UI/InGame/CardDisplay/BP_CardDescriptionStealCardItemWidget.BP_CardDescriptionStealCardItemWidget_C" (Utilities|Array|MakeArray (Class|CardBase|GetIntPropertyDisplayInfo _cardcount)))))))