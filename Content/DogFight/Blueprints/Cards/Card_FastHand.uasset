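; Card_FastHand is a DogFight card Blueprint that targets its own user and increases a card use count by one.
; Its construction script builds the effect by creating InstructionSelectSelf and Instruction_IncreaseOneCardUseCount objects and adding them in that order as instructions.
; GetCardDisplayInfo returns the card's name and description for display, and the event graph holds only disabled default events.
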(event EventBeginPlay)

(event Collision|EventActorBeginOverlap
  (params (OtherActor :type Actor%20Object%20Reference)))

(event EventTick
  (params (DeltaSeconds :type Float%20%28single-precision%29)))

(fn ConstructionScript
  (bind _returnvalue (Game|ConstructObjectfromClass "/Script/DogFight.InstructionSelectSelf" self))
  (Class|CardBase|AddInstruction _returnvalue)
  (bind _returnvalue_2 (Game|ConstructObjectfromClass "/Game/DogFight/Blueprints/Cards/Instructions/Instruction_IncreaseOneCardUseCount.Instruction_IncreaseOneCardUseCount_C" self))
  (Class|CardBase|AddInstruction _returnvalue_2))

(fn GetCardDisplayInfo
  (return (Utilities|Struct|MakeCardInstanceDisplayInfo (Variables|Default|GetCardName) 0 (Variables|Default|GetCardDescription))))