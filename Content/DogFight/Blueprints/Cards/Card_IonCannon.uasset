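; Card Blueprint for the Ion Cannon card in DogFight, pairing a random-point instruction with an ion cannon strike.
; The construction script creates a RandomOnePoint instruction and an IonCannon instruction, keeping a reference to the latter.
; GetCardDisplayInfo builds a localized description from that instruction's upgradable damage, radius and strength cost, shown through a damage-area item widget.
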(event EventBeginPlay)

(event Collision|EventActorBeginOverlap
  (params (OtherActor :type Actor%20Object%20Reference)))

(event EventTick
  (params (DeltaSeconds :type Float%20%28single-precision%29)))

(fn ConstructionScript
  (bind _returnvalue (Game|ConstructObjectfromClass "/Game/DogFight/Blueprints/Cards/Instructions/Instruction_RandomOnePoint.Instruction_RandomOnePoint_C" self))
  (Class|CardBase|AddInstruction _returnvalue)
  (bind _returnvalue_2 (Game|ConstructObjectfromClass "/Game/DogFight/Blueprints/Cards/Instructions/Instruction_IonCannon.Instruction_IonCannon_C" self))
  (bind _output_get (Variables|Default|SetIonCannonInstruction _returnvalue_2))
  (Class|CardBase|AddInstruction _output_get))

(fn GetCardDisplayInfo
  (bind _ioncannoninstruction (Variables|Default|GetIonCannonInstruction))
  (bind _damage (Variables|/Script/DogFight.InstructionSpawnDamageArea|GetDamage _ioncannoninstruction))
  (bind _damageradius (Variables|/Script/DogFight.InstructionSpawnDamageArea|GetDamageRadius _ioncannoninstruction))
  (bind _strengthcost (Variables|/Script/DogFight.InstructionSpawnDamageArea|GetStrengthCost _ioncannoninstruction))
  (return (Utilities|Struct|MakeCardInstanceDisplayInfo (Variables|Default|GetCardName) 0 (Variables|Default|GetCardDescription) 0 (Utilities|Array|MakeArray (Utilities|Struct|MakeCardDescriptionItemInfo "Desc_IonCannon" 0 (Utilities|Array|MakeArray (Utilities|Struct|MakeCardDisplayInfoArgument "Projectile" "Name_IonCannon" "ILT_Projectile" false) (Utilities|Struct|MakeCardDisplayInfoArgument "Default" (Utilities|String|ToString(Integer) (Class|CardBase|GetUpgradableIntPropertyValue _damage)) "ILT_Raw" false) (Utilities|Struct|MakeCardDisplayInfoArgument "Default" "IonDamage" "ILT_Raw" true) (Utilities|Struct|MakeCardDisplayInfoArgument "Default" (Utilities|String|ToString(Integer) (Class|CardBase|GetUpgradableIntPropertyValue _damageradius)) "ILT_Raw" false) (Utilities|Struct|MakeCardDisplayInfoArgument "Default" (Utilities|String|ToString(Integer) (Class|CardBase|GetUpgradableIntPropertyValue _strengthcost)) "ILT_Raw" false)) "ILT_Projectile" "/Game/DogFight/UI/InGame/CardDisplay/BP_CardDescriptionDamageAreaItemWidget.BP_CardDescriptionDamageAreaItemWidget_C" (Utilities|Array|MakeArray (Class|CardBase|GetIntPropertyDisplayInfo _damage) (Class|CardBase|GetIntPropertyDisplayInfo _damageradius) (Class|CardBase|GetIntPropertyDisplayInfo _strengthcost)))))))