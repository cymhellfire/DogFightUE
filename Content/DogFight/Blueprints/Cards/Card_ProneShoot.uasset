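; Card_ProneShoot is a card Blueprint that defines a prone sniper shot on a selected actor as a sequence of instructions.
; Its construction script adds an actor-selection instruction, then a prone-shoot animation instruction.
; The rifle shot is bound to the animation's LaunchProjectile notify as a delegate action, so it fires in step with the animation.
; A similar SpawnActor hook for spawning the rifle is present but unconnected.
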(event EventBeginPlay)

(event Collision|EventActorBeginOverlap
  (params (OtherActor :type Actor%20Object%20Reference)))

(event EventTick
  (params (DeltaSeconds :type Float%20%28single-precision%29)))

(fn ConstructionScript
  (bind _returnvalue (Game|ConstructObjectfromClass "/Game/DogFight/Blueprints/Cards/Instructions/Instruction_SelectOneActor.Instruction_SelectOneActor_C" self))
  (Class|CardBase|AddInstruction _returnvalue)
  (bind _returnvalue_2 (Game|ConstructObjectfromClass "/Game/DogFight/Blueprints/Cards/Instructions/Instruction_AnimProneShoot.Instruction_AnimProneShoot_C" self))
  (bind _output_get (Variables|Default|SetProneShootAnimInstruction _returnvalue_2))
  (Class|CardBase|AddInstruction _output_get)
  (bind _returnvalue_3 (Game|ConstructObjectfromClass "/Game/DogFight/Blueprints/Cards/Instructions/Instruction_SniperRifleShoot.Instruction_SniperRifleShoot_C" self))
  (Class|InstructionPlayAnimation|AddAnimNotifyDelegateAction (Variables|Default|GetProneShootAnimInstruction) (Utilities|Struct|MakeAnimNotifyDelegateAction "DT_LaunchProjectile" 0 _returnvalue_3)))