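; Card Blueprint for a weapon light attack, played against a selected actor.
; The construction script queues two instructions in order: select one actor, then perform the weapon light attack.
; GetCardDisplayInfo adds a light-attack description widget with weapon-localized and raw arguments for standard-mode player controllers, printing an error if the character is invalid.
; Other owners, such as AI players, get only the name and description.
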(event EventBeginPlay)

(event Collision|EventActorBeginOverlap
  (params (OtherActor :type Actor%20Object%20Reference)))

(event EventTick
  (params (DeltaSeconds :type Float%20%28single-precision%29)))

(fn ConstructionScript
  (bind _returnvalue (Game|ConstructObjectfromClass self "/Game/DogFight/Blueprints/Cards/Instructions/Instruction_SelectOneActor.Instruction_SelectOneActor_C"))
  (Class|CardBase|AddInstruction _returnvalue)
  (bind _returnvalue_2 (Game|ConstructObjectfromClass self "/Game/DogFight/Blueprints/Cards/Instructions/Instruction_WeaponLightAttack.Instruction_WeaponLightAttack_C"))
  (Class|CardBase|AddInstruction _returnvalue_2))

(fn GetCardDisplayInfo
  (bind _asstandard_mode_player_controller (Utilities|Casting|CastToStandardModePlayerController (Class|CardBase|GetOwnerPlayerController))
    (:then
      (Utilities|IsValid (Class|GameCardUserPlayerControllerInterface|GetActualPawn _asstandard_mode_player_controller)
        (:Is%20Valid
          (Utilities|Casting|CastToStandardModePlayerCharacter (Class|GameCardUserPlayerControllerInterface|GetActualPawn _asstandard_mode_player_controller)
            (:then
              _)
            (:CastFailed
              (Development|PrintString "Invalid owner character." :!label _label))))
        (:Is%20Not%20Valid
          (goto _label)))
      (return (Utilities|Struct|MakeCardInstanceDisplayInfo (Variables|Default|GetCardName) 0 (Variables|Default|GetCardDescription) 0 (Utilities|Array|MakeArray (Utilities|Struct|MakeCardDescriptionItemInfo "" 0 (Utilities|Array|MakeArray (Utilities|Struct|MakeCardDisplayInfoArgument "Default" "" "ILT_Weapon" false) (Utilities|Struct|MakeCardDisplayInfoArgument "Default" "" "ILT_Weapon" false) (Utilities|Struct|MakeCardDisplayInfoArgument "Default" "" "ILT_Raw" false) (Utilities|Struct|MakeCardDisplayInfoArgument "Default" "" "ILT_Raw" false)) "ILT_Card" "/Game/DogFight/UI/InGame/CardDisplay/BP_CardDescriptionLightAttackItemWidget.BP_CardDescriptionLightAttackItemWidget_C")))))
    (:CastFailed
      ;[1 1 1] Fallback for AI player
      (return (Utilities|Struct|MakeCardInstanceDisplayInfo (Variables|Default|GetCardName) 0 (Variables|Default|GetCardDescription))))))