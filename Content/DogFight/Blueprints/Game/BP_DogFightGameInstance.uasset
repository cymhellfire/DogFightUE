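; BP_DogFightGameInstance is the DogFight game instance Blueprint that handles top-level menu navigation and quitting the game.
; Show events for the main menu, game search, options and profile manager screens lazily create each widget, cache it, then add it to the viewport.
; The card editor opens through the card editor service when that service is valid, rather than through a widget created here.
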(event Custom|ShowSearchGameWidget
  ;[1 1 1] Show Search Game Widget
  (Utilities|IsValid (Variables|Default|GetSearchGameWidget)
    (:Is%20Valid
      _)
    (:Is%20Not%20Valid
      (bind _returnvalue (UserInterface|CreateWidget "/Game/DogFight/UI/Menu/BP_SearchGameWidget.BP_SearchGameWidget_C"))
      (Variables|Default|SetSearchGameWidget _returnvalue)))
  (UserInterface|Viewport|AddtoViewport (Variables|Default|GetSearchGameWidget) 0))

(event Custom|ShowMainMenuWidget
  ;[1 1 1] Show Main Menu Widget
  (Utilities|IsValid (Variables|Default|GetMainMenuWidget)
    (:Is%20Valid
      _)
    (:Is%20Not%20Valid
      (bind _returnvalue (UserInterface|CreateWidget "/Game/DogFight/UI/Menu/BP_MainMenuWidget.BP_MainMenuWidget_C"))
      (Variables|Default|SetMainMenuWidget _returnvalue)))
  (UserInterface|Viewport|AddtoViewport (Variables|Default|GetMainMenuWidget) 0))

(event Custom|QuitGame
  ;[1 1 1] Quit Game
  (Game|QuitGame (Game|GetPlayerController 0) "Quit" false))

(event Custom|ShowOptionsWidget
  ;[1 1 1] Show Options Widget
  (Utilities|IsValid (Variables|Default|GetOptionsWidget)
    (:Is%20Valid
      _)
    (:Is%20Not%20Valid
      (bind _returnvalue (UserInterface|CreateWidget "/Game/DogFight/UI/Menu/BP_OptionsWidget.BP_OptionsWidget_C"))
      (Variables|Default|SetOptionsWidget _returnvalue)))
  (UserInterface|Viewport|AddtoViewport (Variables|Default|GetOptionsWidget) 0))

(event Custom|ShowProfileManagerWidget
  ;[1 1 1] Show Profile Manager
  (Utilities|IsValid (Variables|Default|GetProfileManagerWidget)
    (:Is%20Valid
      _)
    (:Is%20Not%20Valid
      (bind _returnvalue (UserInterface|CreateWidget "/Game/DogFight/UI/Menu/BP_ProfileManagerWidget.BP_ProfileManagerWidget_C"))
      (Variables|Default|SetProfileManagerWidget _returnvalue)))
  (UserInterface|Viewport|AddtoViewport (Variables|Default|GetProfileManagerWidget) 0))

(event Custom|ShowCardEditor
  (bind _returnvalue (Class|CardEditorService|GetCardEditorService))
  (Utilities|IsValid _returnvalue
    (:Is%20Valid
      (Class|CardEditorService|OpenCardEditor _returnvalue))))