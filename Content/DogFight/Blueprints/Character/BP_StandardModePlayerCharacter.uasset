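; Player character Blueprint for standard mode that drives an overhead-style status widget showing the unit's name and health.
; On BeginPlay it casts its WidgetComponent's user widget to BP_PlayerStatusWidget, caches it, and seeds name, max health and current health.
; UnitNameChanged and CurrentHealthChanged events then push updates to the cached widget, guarded by validity checks.
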(event EventBeginPlay
  (bind _asbp_player_status_widget (Utilities|Casting|CastToBP_PlayerStatusWidget (UserInterface|GetUserWidgetObject (Variables|Default|GetWidgetComponent))))
  (bind _output_get (Variables|Default|SetStatusWidget _asbp_player_status_widget))
  (Default|SetPlayerName _output_get (Utilities|Text|ToText(String) (Variables|Default|GetUnitName)))
  (Default|SetPlayerMaxHealth _asbp_player_status_widget (Variables|Default|GetMaxBaseHealth))
  (Default|SetPlayerCurrentHealth _asbp_player_status_widget (Variables|Default|GetCurrentHealth)))

(event EventCurrentHealthChanged
  (params (NewHealth :type Integer))
  (bind _statuswidget (Variables|Default|GetStatusWidget))
  ;[1 1 1] Update the health ratio
  (Utilities|IsValid _statuswidget
    (:Is%20Valid
      (Default|SetPlayerCurrentHealth _statuswidget NewHealth))))

(event EventUnitNameChanged
  (params (PlayerName :type Text%20%28by%20ref%29))
  (bind _statuswidget (Variables|Default|GetStatusWidget))
  ;[1 1 1] Update the player name once it changed
  (Utilities|IsValid _statuswidget
    (:Is%20Valid
      (Default|SetPlayerName _statuswidget PlayerName))))

(fn ConstructionScript)