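; Player controller for DogFight's standard mode, with hard-coded key bindings that exercise game messaging and the card system.
; N broadcasts a greeting game message to all.
; E spawns a BP_Card owned by this controller, assembles it at runtime from wait, select-actor and fire-projectile instruction objects, then uses it immediately.
; The select-actor instruction is outered to the controller, while the other two are outered to the card.
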(event EventBeginPlay)

(event EventTick
  (params (DeltaSeconds :type Float%20%28single-precision%29)))

(event Input|KeyboardEvents|N
  (params (Key :type Key%20Structure :default "None"))
  (:Pressed
    (Class|StandardModePlayerController|CmdBroadcastGameMessagetoAll "GameMsg_Greetings" (Utilities|Array|MakeArray))))

(event Input|KeyboardEvents|E
  (params (Key :type Key%20Structure :default "None"))
  (:Pressed
    (bind _returnvalue (Game|SpawnActorfromClass "/Game/DogFight/Blueprints/Cards/BP_Card.BP_Card_C" (Math|Transform|MakeTransform "0, 0, 0") "Undefined" self (Game|Player|GetPlayerPawn 0)))
    (Class|CardBase|SetOwnerPlayerController _returnvalue self)
    (bind _returnvalue_2 (Game|ConstructObjectfromClass "/Game/DogFight/Blueprints/Cards/Instructions/BP_WaitFor5.BP_WaitFor5_C" _returnvalue))
    (Class|CardBase|AddInstruction _returnvalue _returnvalue_2)
    (bind _returnvalue_3 (Game|ConstructObjectfromClass "/Game/DogFight/Blueprints/Cards/Instructions/BP_SelectActor.BP_SelectActor_C" self))
    (Class|CardBase|AddInstruction _returnvalue _returnvalue_3)
    (bind _returnvalue_4 (Game|ConstructObjectfromClass "/Game/DogFight/Blueprints/Cards/Instructions/BP_FireProjectile.BP_FireProjectile_C" _returnvalue))
    (Class|CardBase|AddInstruction _returnvalue _returnvalue_4)
    (Class|CardBase|Use _returnvalue)))

(fn ConstructionScript)