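; BP_MenuPlayerController is the menu player controller for DogFight, showing the mouse cursor on BeginPlay.
; Its construction script caches the DogFightGameInstance, and hard-coded key events call it to host, find, join or destroy online sessions.
; Two further keys act as debug hooks, one printing a minimum-missing-positive-number test and the other setting the current save game's money to a fixed amount.
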(event EventBeginPlay
  (Variables|Default|SetbShowMouseCursor true))

(event Input|KeyboardEvents|C
  (params (Key :type Key%20Structure :default "None"))
  (bind _gameinstance (Variables|Default|GetGameInstance))
  ;[1 1 1] Host Game
  (:Pressed
    (if (Utilities|IsValid _gameinstance)
      (Class|DogFightGameInstance|HostOnlineGame _gameinstance (Variables|Default|GetGameMapName)))))

(event Input|KeyboardEvents|V
  (params (Key :type Key%20Structure :default "None"))
  (bind _gameinstance (Variables|Default|GetGameInstance))
  ;[1 1 1] Search Games
  (:Pressed
    (if (Utilities|IsValid _gameinstance)
      (Class|DogFightGameInstance|FindOnlineGames _gameinstance))))

(event Input|KeyboardEvents|B
  (params (Key :type Key%20Structure :default "None"))
  (bind _gameinstance (Variables|Default|GetGameInstance))
  ;[1 1 1] Join Game
  (:Pressed
    (if (Utilities|IsValid _gameinstance)
      (Class|DogFightGameInstance|JoinOnlineGame _gameinstance))))

(event Input|KeyboardEvents|N
  (params (Key :type Key%20Structure :default "None"))
  (bind _gameinstance (Variables|Default|GetGameInstance))
  ;[1 1 1] Destroy Session
  (:Pressed
    (if (Utilities|IsValid _gameinstance)
      (Class|DogFightGameInstance|DestroySessionandLeaveGame _gameinstance))))

(event Input|KeyboardEvents|T
  (params (Key :type Key%20Structure :default "None"))
  (:Pressed
    (bind _returnvalue (Class|MathHelperLibrary|GetMinMissingPositiveNumber (Variables|Default|GetTestIntArray) (Variables|Default|GetTestMinNumber)))
    (Development|PrintString (Utilities|String|Append "Result: " (Utilities|String|ToString(Integer) _returnvalue)))))

(event Input|KeyboardEvents|M
  (params (Key :type Key%20Structure :default "None"))
  (:Pressed
    (bind _returnvalue (Class|FrameworkLibrary|GetSaveGameManager))
    (bind _returnvalue_2 (Class|SaveGameManager|GetCurrentSaveGameInstance _returnvalue))
    (Class|DogFightSaveGame|SetMoney _returnvalue_2 500)))

(fn ConstructionScript
  (bind _asdog_fight_game_instance (Utilities|Casting|CastToDogFightGameInstance (Game|GetGameInstance)))
  (Variables|Default|SetGameInstance _asdog_fight_game_instance))