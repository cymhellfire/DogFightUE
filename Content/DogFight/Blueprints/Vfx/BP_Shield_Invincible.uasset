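; BP_Shield_Invincible is a shield effect actor, apparently for an invincibility state in DogFight.
; Its Niagara component plays a spawn effect, then switches to a looping stay asset when the system finishes, tracked by a phase counter.
; Hits on the shield mesh spawn a short-lived BP_Vfx_HolyAuraHit actor at the mesh's location, passing it the impact point and shield scale.
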(event OnComponentHit(ShieldMesh)
  (params (HitComponent :type Primitive%20Component%20Object%20Reference) (OtherActor :type Actor%20Object%20Reference) (OtherComp :type Primitive%20Component%20Object%20Reference) (NormalImpulse :type Vector :default "0, 0, 0") (Hit :type Hit%20Result%20Structure%20%28by%20ref%29))
  (bind _shieldmesh (Variables|Default|GetShieldMesh))
  (bind _returnvalue (Game|SpawnActorfromClass "/Game/DogFight/Blueprints/Vfx/ShieldHit/BP_Vfx_HolyAuraHit.BP_Vfx_HolyAuraHit_C" (Math|Transform|MakeTransform (Transformation|GetWorldLocation _shieldmesh)) "AlwaysSpawn" self (.Location (Collision|BreakHitResult Hit)) (.X (Math|Vector|BreakVector (Transformation|GetWorldScale _shieldmesh))) 0))
  (Actor|SetLifeSpan _returnvalue 5.0))

(event Custom|PlayStayVfx
  (params (PSystem :type Niagara%20Component%20Object%20Reference))
  ;[1 1 1] Play stay Vfx if spawn phase finished
  (if (== (Variables|Default|GetCurrentVfxPhase) 0)
    (Class|NiagaraComponent|SetAsset PSystem (Variables|Default|GetStayVfxAsset))
    (Variables|Default|SetCurrentVfxPhase 1)))

(event EventBeginPlay
  (EventDispatchers|BindEventtoOnSystemFinished (Variables|Default|GetNiagara) (delegate Custom|PlayStayVfx))
  (Variables|Default|SetCurrentVfxPhase 0))

(fn ConstructionScript)