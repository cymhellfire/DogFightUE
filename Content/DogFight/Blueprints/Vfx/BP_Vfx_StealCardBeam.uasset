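; Beam VFX actor for the steal card effect, drawing a Niagara beam from itself toward a target actor.
; Each Tick converts the target's location into the actor's local space and passes it to the beam's TargetPos parameter while the target is valid.
; Events assign the target actor and tint the beam through its CardItemColor variable.
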(event EventOnBeamTargetActorSet
  (params (BeamTargetActor :type Actor%20Object%20Reference))
  (Utilities|IsValid BeamTargetActor
    (:Is%20Valid
      (Variables|Default|SetTargetActor BeamTargetActor))))

(event EventOnCardItemColorSet
  (params (NewColor :type Color%20Structure))
  (Niagara|SetNiagaraVariable(LinearColor) (Variables|Default|GetBeamNiagara) "CardItemColor" (Math|Conversions|ToLinearColor(Color) NewColor)))

(event EventTick
  (params (DeltaSeconds :type Float%20%28single-precision%29))
  (bind _targetactor (Variables|Default|GetTargetActor))
  (Utilities|IsValid _targetactor
    (:Is%20Valid
      (Effects|Components|ParticleSystem|SetVectorParameter (Variables|Default|GetBeamNiagara) "TargetPos" (Math|Transform|InverseTransformLocation (Transformation|GetActorTransform) (Transformation|GetActorLocation _targetactor))))))

(fn ConstructionScript)