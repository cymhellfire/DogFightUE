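; Base Blueprint for a shield hit visual effect in DogFight, shown on a shield mesh at a given hit position.
; The construction script creates a dynamic material instance on the mesh and scales it by ShieldScale.
; On BeginPlay it writes HitPosition into the material, then plays a timeline that drives the material's Phase parameter to animate the hit.
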(event Custom|PlayTimeline
  (bind _hitvfxtime (Timeline|HitTickTimeline PlayFromStart)
    (:Update
      (Rendering|Material|SetScalarParameterValue (Variables|Default|GetMaterialInstance) "Phase" _hitvfxtime :!class /Script/Engine.MaterialInstanceDynamic))))

(event EventBeginPlay
  (Rendering|Material|SetVectorParameterValue (Variables|Default|GetMaterialInstance) "HitPosition" (Math|Conversions|ToLinearColor(Vector) (Variables|Default|GetHitPosition)) :!class /Script/Engine.MaterialInstanceDynamic)
  (CallFunction|PlayTimeline))

(fn ConstructionScript
  (bind _shieldmesh (Variables|Default|GetShieldMesh))
  (bind _returnvalue (Rendering|Material|CreateDynamicMaterialInstance _shieldmesh 0 (Utilities|Array|Get(acopy) (Rendering|Material|GetMaterials _shieldmesh)) "None" :!class /Script/Engine.PrimitiveComponent))
  (bind _output_get (Variables|Default|SetMaterialInstance _returnvalue))
  (Rendering|Material|SetMaterial (Variables|Default|GetShieldMesh) 0 _output_get)
  (Transformation|SetWorldScale3D (Variables|Default|GetShieldMesh) (Math|Conversions|ToVector(Float) (Variables|Default|GetShieldScale))))