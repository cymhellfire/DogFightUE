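; BP_Char_FreeForAll is a character Blueprint, named for a free-for-all mode, that syncs its animation with ragdoll transitions.
; RagdollComponent events drive ThirdPerson_AnimBP on the mesh: activation sets IsDead, caching the pose sets AnimStop, and post-cache calls RecoverFromRagdoll.
; When recovery completes, it stops montages on the anim instance with a short blend-out.
; BeginPlay, Tick, overlap and construction script are empty.
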(event OnRagdollStatusChanged(RagdollComponent)
  (params (bActive :type Boolean))
  ;[1 1 1] Ragdoll Events
  (if bActive
    (Default|SetIsDead (.AsThird%20Person%20Anim%20BP (Utilities|Casting|CastToThirdPerson_AnimBP (Components|SkeletalMesh|GetAnimInstance (Variables|Character|GetMesh)))) true)))

(event OnRagdollCachedPose(RagdollComponent)
  ;[1 1 1] Ragdoll Events
  (Default|SetAnimStop (.AsThird%20Person%20Anim%20BP (Utilities|Casting|CastToThirdPerson_AnimBP (Components|SkeletalMesh|GetAnimInstance (Variables|Character|GetMesh)))) true))

(event PostRagdollCachedPose(RagdollComponent)
  ;[1 1 1] Ragdoll Events
  (Default|RecoverfromRagdoll (.AsThird%20Person%20Anim%20BP (Utilities|Casting|CastToThirdPerson_AnimBP (Components|SkeletalMesh|GetAnimInstance (Variables|Character|GetMesh))))))

(event OnRagdollRecovered(RagdollComponent)
  ;[1 1 1] Ragdoll Events
  (Animation|Montage|MontageStop (Components|SkeletalMesh|GetAnimInstance (Variables|Character|GetMesh)) 0.25 0))

(event EventBeginPlay)

(event Collision|EventActorBeginOverlap
  (params (OtherActor :type Actor%20Object%20Reference)))

(event EventTick
  (params (DeltaSeconds :type Float%20%28single-precision%29)))

(fn ConstructionScript)